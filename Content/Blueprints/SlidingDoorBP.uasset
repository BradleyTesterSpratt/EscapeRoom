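; Sliding door actor that rises when the game instance's ThridTarget flag is set and lowers when it is cleared.
; BeginPlay stores the start position, derives an end position 300 units above it, prints both, and caches the giBP game instance.
; Tick reads the flag every frame and eases the actor toward the matching position with VInterpTo, without sweeping.
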(event EventBeginPlay
  (bind _returnvalue (Transformation|GetActorLocation))
  (bind (_x _y _z) (Math|Vector|BreakVector _returnvalue))
  (bind _returnvalue_2 (+ _z 3e+02))
  (bind _returnvalue_3 (Math|Vector|MakeVector _x _y _returnvalue_2))
  (bind _output_get (Variables|Default|SetStartPos _returnvalue))
  (Development|PrintString (Utilities|String|ToString(Vector) _output_get))
  (Variables|Default|SetEndPos _returnvalue_3)
  (Development|PrintString (Utilities|String|ToString(Vector) _returnvalue_3))
  (bind _asgi_bp (Utilities|Casting|CastTogiBP (Game|GetGameInstance)))
  (Variables|Default|SetgiVar _asgi_bp))

(event EventTick
  (params (DeltaSeconds :type Float%20%28single-precision%29))
  (bind _returnvalue (Transformation|GetActorLocation))
  (bind _returnvalue_2 (Utilities|Time|GetWorldDeltaSeconds))
  (if (Variables|/Game/Blueprints/giBP.giBP_C|GetThridTarget (Variables|Default|GetgiVar))
    (Transformation|SetActorLocation (Math|Interpolation|VInterpTo _returnvalue (Variables|Default|GetEndPos) _returnvalue_2 2.0) false false)
    (else
      (Transformation|SetActorLocation (Math|Interpolation|VInterpTo _returnvalue (Variables|Default|GetStartPos) _returnvalue_2 2.0) false false))))

(fn ConstructionScript)