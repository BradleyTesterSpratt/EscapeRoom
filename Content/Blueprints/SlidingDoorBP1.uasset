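; Sliding door actor that moves vertically between its start position and an offset end position, with StartOpen flipping the direction of travel.
; ToggleDoor picks the destination from the game instance's (giBP) ThirdTarget flag and eases toward it with VInterpTo.
; Tick repeats ToggleDoor only while the door is between both endpoints, so movement from rest needs an external ToggleDoor call.
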(event Custom|toggleDoor
  (if (Variables|/Game/Blueprints/giBP.giBP_C|GetThirdTarget (Variables|Default|GetgiVar))
    (Variables|Default|SetDestinationPos (Variables|Default|GetEndPos))
    (else
      (Variables|Default|SetDestinationPos (Variables|Default|GetStartPos))))
  (Transformation|SetActorLocation (Math|Interpolation|VInterpTo (Transformation|GetActorLocation) (Variables|Default|GetDestinationPos) (Utilities|Time|GetWorldDeltaSeconds) 2.0) false false))

(event EventBeginPlay
  (bind _returnvalue (Transformation|GetActorLocation))
  (bind (_x _y _z) (Math|Vector|BreakVector _returnvalue))
  (if (Variables|UserSettings|GetstartOpen)
    (bind _output_get (Variables|Default|SetEndDirection -2.2e+02))
    (Development|PrintString (Utilities|String|ToString(Float) _output_get))
    (else
      (Variables|Default|SetEndDirection 2.2e+02)))
  (Variables|Default|SetStartPos _returnvalue)
  (Variables|Default|SetEndPos (Math|Vector|MakeVector _x _y (+ _z (Variables|Default|GetEndDirection))))
  (bind _asgi_bp (Utilities|Casting|CastTogiBP (Game|GetGameInstance)))
  (Variables|Default|SetgiVar _asgi_bp))

(event EventTick
  (params (DeltaSeconds :type Float%20%28single-precision%29))
  (bind _returnvalue (Transformation|GetActorLocation))
  (if (not (Math|Vector|Equal(Vector) _returnvalue (Variables|Default|GetStartPos) 0.0001))
    (if (not (Math|Vector|Equal(Vector) _returnvalue (Variables|Default|GetEndPos) 0.0001))
      (CallFunction|ToggleDoor))))

(fn ConstructionScript)