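; A target actor that, when hit, counts toward three simultaneous targets for what appears to be a door unlock.
; A hit swaps to the hit material and reverts after a ten-second delay, ignoring further hits meanwhile.
; Shared booleans in the giBP game instance act as a stacked counter, filled first to third and cleared in reverse.
; Filling the third only prints a door-available message here.
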(event Custom|ToggleOn
  (bind _givar (Variables|Default|GetgiVar))
  (if (Variables|/Game/Blueprints/giBP.giBP_C|GetFirstTarget _givar)
    (if (Variables|/Game/Blueprints/giBP.giBP_C|GetSecondTarget _givar)
      (Variables|/Game/Blueprints/giBP.giBP_C|SetThridTarget _givar true)
      (Development|PrintString "Door Available")
      (else
        (Variables|/Game/Blueprints/giBP.giBP_C|SetSecondTarget _givar true)))
    (else
      (Variables|/Game/Blueprints/giBP.giBP_C|SetFirstTarget _givar true))))

(event Custom|ToggleOff
  (bind _givar (Variables|Default|GetgiVar))
  (if (Variables|/Game/Blueprints/giBP.giBP_C|GetThridTarget _givar)
    (Variables|/Game/Blueprints/giBP.giBP_C|SetThridTarget _givar false)
    (elif (Variables|/Game/Blueprints/giBP.giBP_C|GetSecondTarget _givar)
      (Variables|/Game/Blueprints/giBP.giBP_C|SetSecondTarget _givar false)
      (else
        (Variables|/Game/Blueprints/giBP.giBP_C|SetFirstTarget _givar false)))))

(event EventBeginPlay
  (bind _asgi_bp (Utilities|Casting|CastTogiBP (Game|GetGameInstance)))
  (Variables|Default|SetgiVar _asgi_bp))

(event Collision|EventHit
  (params (MyComp :type Primitive%20Component%20Object%20Reference) (Other :type Actor%20Object%20Reference) (OtherComp :type Primitive%20Component%20Object%20Reference) (bSelfMoved :type Boolean) (HitLocation :type Vector :default "0, 0, 0") (HitNormal :type Vector :default "0, 0, 0") (NormalImpulse :type Vector :default "0, 0, 0") (Hit :type Hit%20Result%20Structure%20%28by%20ref%29))
  (if (not (Variables|Default|GetHit))
    (Variables|Default|SetHit true)
    (CallFunction|Toggleon)
    (Rendering|Material|SetMaterial (Variables|Debug|GetStaticMeshComponent) 0 "/Game/Materials/HitTargetMat.HitTargetMat")
    (Utilities|FlowControl|Delay 1e+01)
    (CallFunction|ToggleOff)
    (Rendering|Material|SetMaterial (Variables|Debug|GetStaticMeshComponent) 0 "/Game/Materials/TargetMat.TargetMat")
    (Variables|Default|SetHit false)))

(fn ConstructionScript)